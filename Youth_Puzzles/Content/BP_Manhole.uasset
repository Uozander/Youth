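; BP_Manhole is a manhole that serves as an entrance to the Lab once an energizer has reached it.
; An overlap of Trigger1 by an actor tagged "energizer" latches the Energizer flag.
; Once latched, a player overlap teleports the player to NewLocation after a short delay, then sets the first-person character's Objective text to finding the sticky hand.
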(event `self.Trigger1.OnComponentBeginOverlap`
  (params (OverlappedComponent :type "PrimitiveComponent Object Reference") (OtherActor :type "Actor Object Reference") (OtherComp :type "PrimitiveComponent Object Reference") (OtherBodyIndex :type Integer) (bFromSweep :type Boolean) (SweepResult :type "HitResult Structure (by ref)"))
  (bind _returnvalue (`GameplayStatics.GetPlayerCharacter` 0))
  (`|ExecutionSequence`
    (:`then_0`
      (if (`self.ActorHasTag` OtherActor "energizer")
        (set `self.Energizer?` true)))
    (:`then_1`
      (if (`self.Energizer?`)
        (if (== OtherActor _returnvalue)
          (`KismetSystemLibrary.Delay` 0.8)
          ;[1 1 1] Entrance to Lab
          (`self.K2_SetActorLocation` _returnvalue (`self.New Location`) false true)
          (bind _asbp_first_person_character (cast `/Game/Characters/Player/Animations/BP_FirstPersonCharacter` _returnvalue))
          (set `/Game/Characters/Player/Animations/BP_FirstPersonCharacter.Objective` "OBJECTIVE - Find the sticky hand" _asbp_first_person_character))))))

(fn `UserConstructionScript`)