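; Bounce pad Blueprint that launches whatever overlaps its Box upward, scaled by BounceFactor.
; For physics components, it adds the negated velocity to the current one, cancelling motion and leaving slight random sideways scatter plus a randomized upward kick.
; If the overlapping actor is BP_FirstPersonCharacter, it also overwrites the movement component's velocity with a fixed, purely vertical launch.
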(event `self.Box.OnComponentBeginOverlap`
  (params (OverlappedComponent :type "PrimitiveComponent Object Reference") (OtherActor :type "Actor Object Reference") (OtherComp :type "PrimitiveComponent Object Reference") (OtherBodyIndex :type Integer) (bFromSweep :type Boolean) (SweepResult :type "HitResult Structure (by ref)"))
  (bind (_returnvalue_x _returnvalue_y _returnvalue_z) (`KismetMathLibrary.BreakVector` (`SceneComponent.GetComponentVelocity` OtherComp)))
  (bind _bounce_factor (`self.Bounce_Factor`))
  (`PrimitiveComponent.SetAllPhysicsLinearVelocity` OtherComp (`KismetMathLibrary.MakeVector` (+ (* _returnvalue_x -1.0) (`KismetMathLibrary.RandomFloatInRange` -50.0 50.0)) (+ (* _returnvalue_y -1.0) (`KismetMathLibrary.RandomFloatInRange` -50.0 50.0)) (+ (* _returnvalue_z -1.0) (`KismetMathLibrary.RandomFloatInRange` _bounce_factor (* _bounce_factor 3.0)))) true)
  (bind _asbp_first_person_character (cast `/Game/Characters/Player/Animations/BP_FirstPersonCharacter` OtherActor))
  (set `MovementComponent.Velocity` (`KismetMathLibrary.MakeVector` 0.0 0.0 (* (`self.Bounce_Factor`) 2.0)) (`Character.CharacterMovement` _asbp_first_person_character)))

(fn `UserConstructionScript`)