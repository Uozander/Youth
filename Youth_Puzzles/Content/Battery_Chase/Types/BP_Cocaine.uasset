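; BP_Cocaine is a moving battery pickup that travels along its own spline.
; On BeginPlay a timeline moves the Sphere component from start to end of the spline via MoveComponentTo, then replays after a random delay.
; When the player overlaps the sphere, it sets the first-person character's Battery flag, shows its battery component and destroys itself.
; Older random-point movement logic remains disconnected, alongside a debug location printer.
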(event `Move_Bug`
  ;[1 1 1] Outside Spline BP
)

(event `Print`
  ;[1 1 1] Print Location
  (`KismetSystemLibrary.PrintString` (`KismetStringLibrary.Conv_VectorToString` (`SceneComponent.K2_GetComponentLocation` (`self.Sphere`))) true true (struct :`R` 1.0 :`G` 0.033202 :`A` 1.0) :!label _label)
  (`KismetSystemLibrary.Delay` 0.5)
  (goto _label))

(event `self.ReceiveBeginPlay`
  (bind _spline (`self.Spline`))
  (`TimelineComponent.SetPlayRate` (`self.TIME_Move`) (/ 1.0 (`self.PlayRate`)))
  (bind (_direction _newtrack_0) (`Timeline|TIME_Move` :!label _label_2)
    (:`Update`
      (bind _returnvalue (`KismetMathLibrary.Lerp` 0.0 (`SplineComponent.GetSplineLength` (`self.Spline`)) _newtrack_0))
      (`KismetSystemLibrary.MoveComponentTo` (`self.Sphere`) (`SplineComponent.GetLocationAtDistanceAlongSpline` _spline _returnvalue "Local") (`SplineComponent.GetRotationAtDistanceAlongSpline` _spline _returnvalue "Local") false false 0.01))
    (:`Finished`
      (`|ExecutionSequence`
        (:`then_0`
          (goto _label_2 :!via `Stop`))
        (:`then_1`
          (`KismetSystemLibrary.Delay` (`KismetMathLibrary.Conv_IntToDouble` (`KismetMathLibrary.RandomIntegerInRange` 0 10)))
          (goto _label_2 :!via `PlayFromStart`))))))

(event `self.Sphere1.OnComponentBeginOverlap`
  (params (OverlappedComponent :type "PrimitiveComponent Object Reference") (OtherActor :type "Actor Object Reference") (OtherComp :type "PrimitiveComponent Object Reference") (OtherBodyIndex :type Integer) (bFromSweep :type Boolean) (SweepResult :type "HitResult Structure (by ref)"))
  (bind _returnvalue (`GameplayStatics.GetPlayerCharacter` 0))
  (if (== OtherActor _returnvalue)
    (bind _asbp_first_person_character (cast `/Game/Characters/Player/Animations/BP_FirstPersonCharacter` _returnvalue))
    (set `/Game/Characters/Player/Animations/BP_FirstPersonCharacter.Battery?` true _asbp_first_person_character)
    (`SceneComponent.SetVisibility` (`/Game/Characters/Player/Animations/BP_FirstPersonCharacter.Battery` _asbp_first_person_character) true false)
    (`self.K2_DestroyActor`)))

(fn `UserConstructionScript`)