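; BP_Battery1 is a battery pickup that moves along a spline for the player to catch.
; On BeginPlay, a timeline with a play rate set from PlayRate drives the actor's location and rotation by distance along the spline.
; When the player overlaps its sphere, it sets the first-person character's battery flag, shows that character's battery and destroys itself.
; An older random-waypoint movement remains unconnected.
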(event `Move_Bug`)

(event `self.ReceiveBeginPlay`
  (bind _spline (`self.Spline`))
  (`TimelineComponent.SetPlayRate` (`self.TIME_Move`) (/ 1.0 (`self.Play Rate`)))
  (bind (_direction _newtrack_0) (`Timeline|TIME_Move`)
    (:`Update`
      (bind _returnvalue (`KismetMathLibrary.Lerp` 0.0 (`SplineComponent.GetSplineLength` (`self.Spline`)) _newtrack_0))
      (`self.K2_SetActorTransform` (`KismetMathLibrary.MakeTransform` (`SplineComponent.GetLocationAtDistanceAlongSpline` _spline _returnvalue "World") (`SplineComponent.GetRotationAtDistanceAlongSpline` _spline _returnvalue "Local"))))))

(event `self.Sphere1.OnComponentBeginOverlap`
  (params (OverlappedComponent :type "PrimitiveComponent Object Reference") (OtherActor :type "Actor Object Reference") (OtherComp :type "PrimitiveComponent Object Reference") (OtherBodyIndex :type Integer) (bFromSweep :type Boolean) (SweepResult :type "HitResult Structure (by ref)"))
  (bind _returnvalue (`GameplayStatics.GetPlayerCharacter` 0))
  (if (== OtherActor _returnvalue)
    (bind _asbp_first_person_character (cast `/Game/Characters/Player/Animations/BP_FirstPersonCharacter` _returnvalue))
    (set `/Game/Characters/Player/Animations/BP_FirstPersonCharacter.Battery?` true _asbp_first_person_character)
    (`SceneComponent.SetVisibility` (`/Game/Characters/Player/Animations/BP_FirstPersonCharacter.Battery` _asbp_first_person_character) true false)
    (`self.K2_DestroyActor`)))

(fn `UserConstructionScript`)