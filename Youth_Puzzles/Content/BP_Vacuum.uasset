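; BP_Vacuum is a trigger actor that lifts the player character straight up while inside its W component's overlap area.
; Begin overlap sets a flag and starts a short Delay loop that repeatedly calls LaunchCharacter with a fixed upward velocity until end overlap clears it.
; Each launch overrides all axes, cancelling horizontal momentum; a gentler additive launch, noted as less controlled, is left unconnected.
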(event `self.w.OnComponentBeginOverlap`
  (params (OverlappedComponent :type "PrimitiveComponent Object Reference") (OtherActor :type "Actor Object Reference") (OtherComp :type "PrimitiveComponent Object Reference") (OtherBodyIndex :type Integer) (bFromSweep :type Boolean) (SweepResult :type "HitResult Structure (by ref)"))
  (if (== OtherActor (`GameplayStatics.GetPlayerCharacter` 0))
    (set `self.Overlap?` true)
    (if (`self.Overlap?`) :!label _label
      (`Character.LaunchCharacter` (`GameplayStatics.GetPlayerCharacter` 0) (0.0 0.0 400.0) true true)
      (`KismetSystemLibrary.Delay` 0.01)
      (goto _label))))

(event `self.w.OnComponentEndOverlap`
  (params (OverlappedComponent :type "PrimitiveComponent Object Reference") (OtherActor :type "Actor Object Reference") (OtherComp :type "PrimitiveComponent Object Reference") (OtherBodyIndex :type Integer))
  (if (== OtherActor (`GameplayStatics.GetPlayerCharacter` 0))
    (set `self.Overlap?` false)))

(fn `UserConstructionScript`)