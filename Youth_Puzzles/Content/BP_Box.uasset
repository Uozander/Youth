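; BP_Box is a box Blueprint that makes the player drop their grabbed blocks when it collides while held.
; When its Button component hits anything not exactly of class BP_Piece while Held is true, it reads GrabbedBlocks from BP_FirstPersonCharacter.
; It clears Held on each block's owning BP_Piece, re-enables gravity on the grabbed component, then empties the array.
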(event `self.Button.OnComponentHit`
  (params (HitComponent :type "PrimitiveComponent Object Reference") (OtherActor :type "Actor Object Reference") (OtherComp :type "PrimitiveComponent Object Reference") (NormalImpulse :type "Vector Structure") (Hit :type "HitResult Structure (by ref)"))
  (if (`self.Held?`)
    (if (not (== (`GameplayStatics.GetObjectClass` OtherActor) "/Game/Puzzles/BP_Piece.BP_Piece_C"))
      (bind _asbp_first_person_character (cast `/Game/Characters/Player/Animations/BP_FirstPersonCharacter` (`GameplayStatics.GetPlayerCharacter` 0)))
      (bind _grabbed_blocks (`/Game/Characters/Player/Animations/BP_FirstPersonCharacter.Grabbed_Blocks` _asbp_first_person_character))
      (for _array_element _grabbed_blocks
        (bind _asbp_piece (cast `/Game/Puzzles/BP_Piece` (`ActorComponent.GetOwner` _array_element)))
        (set `/Game/Puzzles/BP_Piece.Held?` false _asbp_piece)
        (`PrimitiveComponent.SetEnableGravity` _array_element true))
      (`KismetArrayLibrary.Array_Clear` _grabbed_blocks))))

(fn `UserConstructionScript`)