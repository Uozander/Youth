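; BP_Obelisk is an obelisk with four slots that accept a piece in the correct orientation.
; Each box trigger checks an overlapping component for the "speak" tag and an exact world roll, upright for two slots and flipped for the other two.
; A match reveals that slot's mesh, hides the first-person character's Piece component and destroys the trigger, so each slot fills once.
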(event `self.Box.OnComponentBeginOverlap`
  (params (OverlappedComponent :type "PrimitiveComponent Object Reference") (OtherActor :type "Actor Object Reference") (OtherComp :type "PrimitiveComponent Object Reference") (OtherBodyIndex :type Integer) (bFromSweep :type Boolean) (SweepResult :type "HitResult Structure (by ref)"))
  (bind _returnvalue_roll (`KismetMathLibrary.BreakRotator` (`SceneComponent.K2_GetComponentRotation` OtherComp)))
  (if (`ActorComponent.ComponentHasTag` OtherComp "speak")
    (if (== _returnvalue_roll 180.0)
      (`SceneComponent.SetVisibility` (`self.StaticMesh1`) true false)
      (bind _asbp_first_person_character (cast `/Game/FirstPerson/Blueprints/BP_FirstPersonCharacter` (`GameplayStatics.GetPlayerCharacter` 0)))
      (`SceneComponent.SetVisibility` (`/Game/FirstPerson/Blueprints/BP_FirstPersonCharacter.Piece` _asbp_first_person_character) false false)
      (`ActorComponent.K2_DestroyComponent` (`self.Box`)))))

(event `self.Box3.OnComponentBeginOverlap`
  (params (OverlappedComponent :type "PrimitiveComponent Object Reference") (OtherActor :type "Actor Object Reference") (OtherComp :type "PrimitiveComponent Object Reference") (OtherBodyIndex :type Integer) (bFromSweep :type Boolean) (SweepResult :type "HitResult Structure (by ref)"))
  (bind _returnvalue_roll (`KismetMathLibrary.BreakRotator` (`SceneComponent.K2_GetComponentRotation` OtherComp)))
  (if (`ActorComponent.ComponentHasTag` OtherComp "speak")
    (if (== _returnvalue_roll 180.0)
      (`SceneComponent.SetVisibility` (`self.StaticMesh3`) true false)
      (bind _asbp_first_person_character (cast `/Game/FirstPerson/Blueprints/BP_FirstPersonCharacter` (`GameplayStatics.GetPlayerCharacter` 0)))
      (`SceneComponent.SetVisibility` (`/Game/FirstPerson/Blueprints/BP_FirstPersonCharacter.Piece` _asbp_first_person_character) false false)
      (`ActorComponent.K2_DestroyComponent` (`self.Box3`)))))

(event `self.Box1.OnComponentBeginOverlap`
  (params (OverlappedComponent :type "PrimitiveComponent Object Reference") (OtherActor :type "Actor Object Reference") (OtherComp :type "PrimitiveComponent Object Reference") (OtherBodyIndex :type Integer) (bFromSweep :type Boolean) (SweepResult :type "HitResult Structure (by ref)"))
  (bind _returnvalue_roll (`KismetMathLibrary.BreakRotator` (`SceneComponent.K2_GetComponentRotation` OtherComp)))
  (if (`ActorComponent.ComponentHasTag` OtherComp "speak")
    (if (== _returnvalue_roll 0.0)
      (`SceneComponent.SetVisibility` (`self.StaticMesh2`) true false)
      (bind _asbp_first_person_character (cast `/Game/FirstPerson/Blueprints/BP_FirstPersonCharacter` (`GameplayStatics.GetPlayerCharacter` 0)))
      (`SceneComponent.SetVisibility` (`/Game/FirstPerson/Blueprints/BP_FirstPersonCharacter.Piece` _asbp_first_person_character) false false)
      (`ActorComponent.K2_DestroyComponent` (`self.Box1`)))))

(event `self.Box2.OnComponentBeginOverlap`
  (params (OverlappedComponent :type "PrimitiveComponent Object Reference") (OtherActor :type "Actor Object Reference") (OtherComp :type "PrimitiveComponent Object Reference") (OtherBodyIndex :type Integer) (bFromSweep :type Boolean) (SweepResult :type "HitResult Structure (by ref)"))
  (bind _returnvalue_roll (`KismetMathLibrary.BreakRotator` (`SceneComponent.K2_GetComponentRotation` OtherComp)))
  (if (`ActorComponent.ComponentHasTag` OtherComp "speak")
    (if (== _returnvalue_roll 0.0)
      (`SceneComponent.SetVisibility` (`self.StaticMesh4`) true false)
      (bind _asbp_first_person_character (cast `/Game/FirstPerson/Blueprints/BP_FirstPersonCharacter` (`GameplayStatics.GetPlayerCharacter` 0)))
      (`SceneComponent.SetVisibility` (`/Game/FirstPerson/Blueprints/BP_FirstPersonCharacter.Piece` _asbp_first_person_character) false false)
      (`ActorComponent.K2_DestroyComponent` (`self.Box2`)))))

(fn `UserConstructionScript`)