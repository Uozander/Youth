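; BP_Sticky_Object1 is a short-lived sticky object that traps the first-person player on contact and destroys itself after a fixed lifetime.
; When the player overlaps its box, a brief delay precedes zeroing the character's gravity scale and velocity, setting its Stuck flag and destroying the object.
; End overlap does nothing; older gravity-restoring logic remains disconnected, so the object never releases the player itself.
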(event `self.ReceiveBeginPlay`
  (`KismetSystemLibrary.Delay` 20.0)
  (`self.K2_DestroyActor`))

(event `self.Box.OnComponentBeginOverlap`
  (params (OverlappedComponent :type "PrimitiveComponent Object Reference") (OtherActor :type "Actor Object Reference") (OtherComp :type "PrimitiveComponent Object Reference") (OtherBodyIndex :type Integer) (bFromSweep :type Boolean) (SweepResult :type "HitResult Structure (by ref)"))
  (bind _returnvalue (`GameplayStatics.GetPlayerCharacter` 0))
  (if (== OtherActor _returnvalue)
    (bind _asbp_first_person_character (cast `/Game/Characters/Player/Animations/BP_FirstPersonCharacter` _returnvalue))
    (`KismetSystemLibrary.Delay` 0.2)
    (bind _charactermovement (`Character.CharacterMovement` _asbp_first_person_character))
    (set `CharacterMovementComponent.GravityScale` 0.0 _charactermovement)
    (set `MovementComponent.Velocity` (0.0 0.0 0.0) _charactermovement)
    (set `/Game/Characters/Player/Animations/BP_FirstPersonCharacter.Stuck?` true _asbp_first_person_character)
    (`self.K2_DestroyActor`)))

(event `self.Box.OnComponentEndOverlap`
  (params (OverlappedComponent :type "PrimitiveComponent Object Reference") (OtherActor :type "Actor Object Reference") (OtherComp :type "PrimitiveComponent Object Reference") (OtherBodyIndex :type Integer)))

(fn `UserConstructionScript`)