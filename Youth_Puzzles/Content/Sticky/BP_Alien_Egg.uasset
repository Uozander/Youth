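; Alien egg pickup that grants the player the sticky hand.
; Any overlap with Box1 starts an endless delay-loop yaw spin on the skeletal mesh and eases it to a relative height over one second.
; When the player overlaps Box, it sets the StickyHand flag on BP_FirstPersonCharacter, updates the objective to reaching the vent, then destroys itself.
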(event `self.Box1.OnComponentBeginOverlap`
  (params (OverlappedComponent :type "PrimitiveComponent Object Reference") (OtherActor :type "Actor Object Reference") (OtherComp :type "PrimitiveComponent Object Reference") (OtherBodyIndex :type Integer) (bFromSweep :type Boolean) (SweepResult :type "HitResult Structure (by ref)"))
  (`|ExecutionSequence`
    (:`then_0`
      ;[1 1 1] Spin StickyHand
      (`KismetSystemLibrary.Delay` 0.01 :!label _label)
      (bind _output_get (set `self.rotation` (+ (`self.rotation`) 10.0)))
      (`SceneComponent.K2_SetWorldRotation` (`self.SkeletalMesh`) (`KismetMathLibrary.MakeRotator` 0.0 0.0 _output_get) false false)
      (goto _label))
    (:`then_1`
      (`KismetSystemLibrary.MoveComponentTo` (`self.SkeletalMesh`) (0.0 0.0 100.0) (struct) true true 1.0))))

(event `self.Box.OnComponentBeginOverlap`
  (params (OverlappedComponent :type "PrimitiveComponent Object Reference") (OtherActor :type "Actor Object Reference") (OtherComp :type "PrimitiveComponent Object Reference") (OtherBodyIndex :type Integer) (bFromSweep :type Boolean) (SweepResult :type "HitResult Structure (by ref)"))
  (bind _returnvalue (`GameplayStatics.GetPlayerCharacter` 0))
  (if (== OtherActor _returnvalue)
    (bind _asbp_first_person_character (cast `/Game/Characters/Player/Animations/BP_FirstPersonCharacter` _returnvalue))
    (set `/Game/Characters/Player/Animations/BP_FirstPersonCharacter.StickyHand?` true _asbp_first_person_character)
    (set `/Game/Characters/Player/Animations/BP_FirstPersonCharacter.Objective` "OBJECTIVE - Use sticky hand to reach the vent" _asbp_first_person_character)
    (`self.K2_DestroyActor`)))

(fn `UserConstructionScript`)