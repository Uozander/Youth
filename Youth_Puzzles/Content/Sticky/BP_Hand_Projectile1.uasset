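; BP_Hand_Projectile1 is a sticky hand projectile that stops where it first hits something.
; A one-shot hit event rotates the hand mesh from a hit-derived vector, waits briefly, then zeroes gravity and velocity and disables collision and physics.
; The "sticky" tag check is unwired, so it sticks to any surface, and debug prints remain.
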(event `self.stickyhand_collision.OnComponentHit`
  (params (HitComponent :type "PrimitiveComponent Object Reference") (OtherActor :type "Actor Object Reference") (OtherComp :type "PrimitiveComponent Object Reference") (NormalImpulse :type "Vector Structure") (Hit :type "HitResult Structure (by ref)"))
  (bind _projectilemovement (`self.ProjectileMovement`))
  (bind _stickyhand_collision (`self.stickyhand_collision`))
  (`/Engine/EditorBlueprintResources/StandardMacros.DoOnce` false
    (:`Completed`
      (`KismetSystemLibrary.PrintString` (`KismetSystemLibrary.GetDisplayName` OtherComp))
      (if true
        (`SceneComponent.K2_SetRelativeRotation` (`self.stickyhand_mesh`) (`KismetMathLibrary.Conv_VectorToRotator` (`.ImpactNormal` (`GameplayStatics.BreakHitResult` Hit))) false false)
        (`KismetSystemLibrary.Delay` 0.03)
        (set `ProjectileMovementComponent.ProjectileGravityScale` 0.0 _projectilemovement)
        (set `MovementComponent.Velocity` (0.0 0.0 0.0) _projectilemovement)
        (`PrimitiveComponent.SetSimulatePhysics` _stickyhand_collision false)
        (`PrimitiveComponent.SetCollisionEnabled` _stickyhand_collision "NoCollision")
        (`KismetSystemLibrary.PrintString` "Hello")))))

(fn `UserConstructionScript`)