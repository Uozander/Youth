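; Ice surface puzzle piece that makes the first-person character slide while inside its Box trigger.
; Entering the box zeroes the character's ground friction and braking and cuts walk speed to almost nothing, so existing momentum carries it along.
; Leaving waits briefly, then sets fixed movement values rather than cached originals, with braking deceleration copied from the low braking friction factor.
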(event `self.Box.OnComponentBeginOverlap`
  (params (OverlappedComponent :type "PrimitiveComponent Object Reference") (OtherActor :type "Actor Object Reference") (OtherComp :type "PrimitiveComponent Object Reference") (OtherBodyIndex :type Integer) (bFromSweep :type Boolean) (SweepResult :type "HitResult Structure (by ref)"))
  (bind _asbp_first_person_character (cast `/Game/Characters/Player/Animations/BP_FirstPersonCharacter` OtherActor))
  (bind _charactermovement (`Character.CharacterMovement` _asbp_first_person_character))
  (set `CharacterMovementComponent.GroundFriction` 0.0 _charactermovement)
  (set `CharacterMovementComponent.BrakingFrictionFactor` 0.0 _charactermovement)
  (set `CharacterMovementComponent.BrakingDecelerationWalking` 0.0 _charactermovement)
  (set `CharacterMovementComponent.MaxWalkSpeed` 10.0 _charactermovement))

(event `self.Box.OnComponentEndOverlap`
  (params (OverlappedComponent :type "PrimitiveComponent Object Reference") (OtherActor :type "Actor Object Reference") (OtherComp :type "PrimitiveComponent Object Reference") (OtherBodyIndex :type Integer))
  (bind _asbp_first_person_character (cast `/Game/Characters/Player/Animations/BP_FirstPersonCharacter` OtherActor))
  (`KismetSystemLibrary.Delay` 0.2)
  (bind _charactermovement (`Character.CharacterMovement` _asbp_first_person_character))
  (set `CharacterMovementComponent.GroundFriction` 8.0 _charactermovement)
  (bind _output_get (set `CharacterMovementComponent.BrakingFrictionFactor` 2.0 _charactermovement))
  (set `CharacterMovementComponent.BrakingDecelerationWalking` _output_get _charactermovement)
  (set `CharacterMovementComponent.MaxWalkSpeed` 600.0 _charactermovement))

(fn `UserConstructionScript`)