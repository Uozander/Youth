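; BP_Piece is a grabbable puzzle piece with a Button component and a light.
; When a held piece hits anything that is not a BP_Piece, it releases every block in the first-person character's GrabbedBlocks, restoring gravity and clearing the list.
; CE_Bloom briefly swaps the Button material behind a resetting DoOnce.
; Tick scales the light's intensity by player distance within the glow range, dimming it as the player approaches.
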(event `CE_Bloom`
  (`/Engine/EditorBlueprintResources/StandardMacros.DoOnce` false :!label _label
    (:`Completed`
      (`PrimitiveComponent.SetMaterial` (`self.Button`) 0 "/Game/Puzzles/Obelisk/Button/LETTER_A/MAT_AND_LETTER_A_Inst.MAT_AND_LETTER_A_Inst")
      (`KismetSystemLibrary.Delay` 0.5)
      (`PrimitiveComponent.SetMaterial` (`self.Button`) 0 "/Game/Puzzles/Obelisk/Button/LETTER_A/MAT_AND_LETTER_A.MAT_AND_LETTER_A")
      (goto _label :!via `Reset`))))

(event `self.Button.OnComponentHit`
  (params (HitComponent :type "PrimitiveComponent Object Reference") (OtherActor :type "Actor Object Reference") (OtherComp :type "PrimitiveComponent Object Reference") (NormalImpulse :type "Vector Structure") (Hit :type "HitResult Structure (by ref)"))
  (if (`self.Held?`)
    (if (not (== (`GameplayStatics.GetObjectClass` OtherActor) "BP_Piece_C"))
      (bind _asbp_first_person_character (cast `/Game/Characters/Player/Animations/BP_FirstPersonCharacter` (`GameplayStatics.GetPlayerCharacter` 0)))
      (bind _grabbed_blocks (`/Game/Characters/Player/Animations/BP_FirstPersonCharacter.Grabbed_Blocks` _asbp_first_person_character))
      (for _array_element _grabbed_blocks
        (bind _asbp_piece (cast `/Game/Puzzles/BP_Piece` (`ActorComponent.GetOwner` _array_element)))
        (set `/Game/Puzzles/BP_Piece.Held?` false _asbp_piece)
        (`PrimitiveComponent.SetEnableGravity` _array_element true))
      (`KismetArrayLibrary.Array_Clear` _grabbed_blocks))))

(event `self.ReceiveTick`
  (params (DeltaSeconds :type "Float (single-precision)"))
  (bind _disntance_glow (`self.Disntance Glow`))
  (bind _returnvalue (`KismetMathLibrary.Vector_Distance` (`SceneComponent.K2_GetComponentLocation` (`self.Button`)) (`self.K2_GetActorLocation` (`GameplayStatics.GetPlayerCharacter` 0))))
  (`/Engine/EditorBlueprintResources/StandardMacros.IsValid` (`self.ButtonLight`)
    (:`Is Valid`
      (if (< _returnvalue _disntance_glow)
        (`LightComponent.SetIntensity` (`self.ButtonLight`) (* (`self.Intensity`) (`KismetMathLibrary.NormalizeToRange` _returnvalue (`self.Distance Offset`) _disntance_glow)))))))

(fn `UserConstructionScript`)