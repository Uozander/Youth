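; Obelisk puzzle actor with five sockets, where the player docks held pieces to trigger the ending.
; Each trigger box reacts to a "speak"-tagged component while the character's Held flag is set, clearing it, revealing that socket's button mesh and destroying itself.
; Each placement increments the piece and character counters, resets the UI and plays a staggered sound sequence.
; At five pieces it plays a final sting and calls CallEDEND.
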(event `self.Box6.OnComponentBeginOverlap`
  (params (OverlappedComponent :type "PrimitiveComponent Object Reference") (OtherActor :type "Actor Object Reference") (OtherComp :type "PrimitiveComponent Object Reference") (OtherBodyIndex :type Integer) (bFromSweep :type Boolean) (SweepResult :type "HitResult Structure (by ref)"))
  (bind _returnvalue (`self.K2_GetActorLocation`))
  (if (`ActorComponent.ComponentHasTag` OtherComp "speak")
    (bind _asbp_first_person_character (cast `/Game/Characters/Player/Animations/BP_FirstPersonCharacter` (`GameplayStatics.GetPlayerCharacter` 0)))
    (if (`/Game/Characters/Player/Animations/BP_FirstPersonCharacter.Held?` _asbp_first_person_character)
      (set `/Game/Characters/Player/Animations/BP_FirstPersonCharacter.Held?` false _asbp_first_person_character)
      (`SceneComponent.SetVisibility` (`/Game/Characters/Player/Animations/BP_FirstPersonCharacter.StickyTarget2` _asbp_first_person_character) false false)
      (`SceneComponent.SetVisibility` (`self.Button21`) true false)
      (`ActorComponent.K2_DestroyComponent` (`self.Box6`))
      (set `self.Obelisk_Pieces` (+ (`self.Obelisk_Pieces`) 1))
      (set `/Game/Characters/Player/Animations/BP_FirstPersonCharacter.SnS_Count` (+ (`/Game/Characters/Player/Animations/BP_FirstPersonCharacter.SnS_Count` _asbp_first_person_character) 1) _asbp_first_person_character)
      (`/Game/Characters/Player/Animations/BP_FirstPersonCharacter.CE_ResetUI` _asbp_first_person_character)
      (`GameplayStatics.PlaySoundAtLocation` "/Engine/VREditor/Sounds/UI/Dockable_Window_Drop.Dockable_Window_Drop" _returnvalue (struct) 1.0 1.0 0.0 null null null null :!label _label)
      (`KismetSystemLibrary.Delay` 0.5)
      (`GameplayStatics.PlaySoundAtLocation` "/Game/Puzzles/Obelisk/Alien_BUCKET.Alien_BUCKET" _returnvalue (struct) 1.0 1.0 0.0 null null null null)
      (`KismetSystemLibrary.Delay` 1.0)
      (`GameplayStatics.PlaySoundAtLocation` "/Game/Puzzles/Obelisk/Human_BUCKET.Human_BUCKET" _returnvalue (struct) 1.0 1.0 0.0 null null null null)
      (if (>= (`self.Obelisk_Pieces`) 5)
        (`GameplayStatics.PlaySound2D` "/Game/Sounds/Final_Cat_Studio_-_Its_Magic_-_Ethereal_Logo_Reveal.Final_Cat_Studio_-_Its_Magic_-_Ethereal_Logo_Reveal" 1.0 1.0 0.0 null null)
        (`self.ED_END`)))))

(event `self.Box.OnComponentBeginOverlap`
  (params (OverlappedComponent :type "PrimitiveComponent Object Reference") (OtherActor :type "Actor Object Reference") (OtherComp :type "PrimitiveComponent Object Reference") (OtherBodyIndex :type Integer) (bFromSweep :type Boolean) (SweepResult :type "HitResult Structure (by ref)"))
  (if (`ActorComponent.ComponentHasTag` OtherComp "speak")
    (bind _asbp_first_person_character (cast `/Game/Characters/Player/Animations/BP_FirstPersonCharacter` (`GameplayStatics.GetPlayerCharacter` 0)))
    (if (`/Game/Characters/Player/Animations/BP_FirstPersonCharacter.Held?` _asbp_first_person_character)
      (set `/Game/Characters/Player/Animations/BP_FirstPersonCharacter.Held?` false _asbp_first_person_character)
      (`SceneComponent.SetVisibility` (`/Game/Characters/Player/Animations/BP_FirstPersonCharacter.StickyTarget2` _asbp_first_person_character) false false)
      (`SceneComponent.SetVisibility` (`self.Button17`) true false)
      (`ActorComponent.K2_DestroyComponent` (`self.Box`))
      (set `self.Obelisk_Pieces` (+ (`self.Obelisk_Pieces`) 1))
      (set `/Game/Characters/Player/Animations/BP_FirstPersonCharacter.SnS_Count` (+ (`/Game/Characters/Player/Animations/BP_FirstPersonCharacter.SnS_Count` _asbp_first_person_character) 1) _asbp_first_person_character)
      (`/Game/Characters/Player/Animations/BP_FirstPersonCharacter.CE_ResetUI` _asbp_first_person_character)
      (goto _label))))

(event `self.Box3.OnComponentBeginOverlap`
  (params (OverlappedComponent :type "PrimitiveComponent Object Reference") (OtherActor :type "Actor Object Reference") (OtherComp :type "PrimitiveComponent Object Reference") (OtherBodyIndex :type Integer) (bFromSweep :type Boolean) (SweepResult :type "HitResult Structure (by ref)"))
  (if (`ActorComponent.ComponentHasTag` OtherComp "speak")
    (bind _asbp_first_person_character (cast `/Game/Characters/Player/Animations/BP_FirstPersonCharacter` (`GameplayStatics.GetPlayerCharacter` 0)))
    (if (`/Game/Characters/Player/Animations/BP_FirstPersonCharacter.Held?` _asbp_first_person_character)
      (set `/Game/Characters/Player/Animations/BP_FirstPersonCharacter.Held?` false _asbp_first_person_character)
      (`SceneComponent.SetVisibility` (`/Game/Characters/Player/Animations/BP_FirstPersonCharacter.StickyTarget2` _asbp_first_person_character) false false)
      (`SceneComponent.SetVisibility` (`self.Button20`) true false)
      (`ActorComponent.K2_DestroyComponent` (`self.Box3`))
      (set `self.Obelisk_Pieces` (+ (`self.Obelisk_Pieces`) 1))
      (set `/Game/Characters/Player/Animations/BP_FirstPersonCharacter.SnS_Count` (+ (`/Game/Characters/Player/Animations/BP_FirstPersonCharacter.SnS_Count` _asbp_first_person_character) 1) _asbp_first_person_character)
      (`/Game/Characters/Player/Animations/BP_FirstPersonCharacter.CE_ResetUI` _asbp_first_person_character)
      (goto _label))))

(event `self.Box1.OnComponentBeginOverlap`
  (params (OverlappedComponent :type "PrimitiveComponent Object Reference") (OtherActor :type "Actor Object Reference") (OtherComp :type "PrimitiveComponent Object Reference") (OtherBodyIndex :type Integer) (bFromSweep :type Boolean) (SweepResult :type "HitResult Structure (by ref)"))
  (if (`ActorComponent.ComponentHasTag` OtherComp "speak")
    (bind _asbp_first_person_character (cast `/Game/Characters/Player/Animations/BP_FirstPersonCharacter` (`GameplayStatics.GetPlayerCharacter` 0)))
    (if (`/Game/Characters/Player/Animations/BP_FirstPersonCharacter.Held?` _asbp_first_person_character)
      (set `/Game/Characters/Player/Animations/BP_FirstPersonCharacter.Held?` false _asbp_first_person_character)
      (`SceneComponent.SetVisibility` (`/Game/Characters/Player/Animations/BP_FirstPersonCharacter.StickyTarget2` _asbp_first_person_character) false false)
      (`SceneComponent.SetVisibility` (`self.Button18`) true false)
      (`ActorComponent.K2_DestroyComponent` (`self.Box1`))
      (set `self.Obelisk_Pieces` (+ (`self.Obelisk_Pieces`) 1))
      (set `/Game/Characters/Player/Animations/BP_FirstPersonCharacter.SnS_Count` (+ (`/Game/Characters/Player/Animations/BP_FirstPersonCharacter.SnS_Count` _asbp_first_person_character) 1) _asbp_first_person_character)
      (`/Game/Characters/Player/Animations/BP_FirstPersonCharacter.CE_ResetUI` _asbp_first_person_character)
      (goto _label))))

(event `self.Box2.OnComponentBeginOverlap`
  (params (OverlappedComponent :type "PrimitiveComponent Object Reference") (OtherActor :type "Actor Object Reference") (OtherComp :type "PrimitiveComponent Object Reference") (OtherBodyIndex :type Integer) (bFromSweep :type Boolean) (SweepResult :type "HitResult Structure (by ref)"))
  (if (`ActorComponent.ComponentHasTag` OtherComp "speak")
    (bind _asbp_first_person_character (cast `/Game/Characters/Player/Animations/BP_FirstPersonCharacter` (`GameplayStatics.GetPlayerCharacter` 0)))
    (if (`/Game/Characters/Player/Animations/BP_FirstPersonCharacter.Held?` _asbp_first_person_character)
      (set `/Game/Characters/Player/Animations/BP_FirstPersonCharacter.Held?` false _asbp_first_person_character)
      (`SceneComponent.SetVisibility` (`/Game/Characters/Player/Animations/BP_FirstPersonCharacter.StickyTarget2` _asbp_first_person_character) false false)
      (`SceneComponent.SetVisibility` (`self.Button19`) true false)
      (`ActorComponent.K2_DestroyComponent` (`self.Box2`))
      (set `self.Obelisk_Pieces` (+ (`self.Obelisk_Pieces`) 1))
      (set `/Game/Characters/Player/Animations/BP_FirstPersonCharacter.SnS_Count` (+ (`/Game/Characters/Player/Animations/BP_FirstPersonCharacter.SnS_Count` _asbp_first_person_character) 1) _asbp_first_person_character)
      (`/Game/Characters/Player/Animations/BP_FirstPersonCharacter.CE_ResetUI` _asbp_first_person_character)
      (goto _label))))

(fn `UserConstructionScript`)