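; BP_Battery is a battery pickup for the Battery Chase puzzle that keeps moving between predefined points until the player touches it.
; A timeline lerps it from its current location toward a transform in BatteryTransforms, then a random reroll picks an index different from the last.
; Overlapping the player with its sphere sets the first-person character's Battery flag, shows its Battery component and destroys the pickup.
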(event `self.ReceiveBeginPlay`
  (bind _current_integer (`self.Current Integer`))
  (bind _output_location (`KismetMathLibrary.BreakTransform` (`|GetArrayItem` (`self.Battery Transforms`) _current_integer)))
  (set `self.Location` _output_location :!label _label)
  (bind (_direction _newtrack_2) (`Timeline|Timeline` :!via `PlayFromStart`)
    (:`Update`
      (`self.K2_SetActorLocation` (`KismetMathLibrary.VLerp` (`self.K2_GetActorLocation`) (`self.Location`) _newtrack_2)))
    (:`Finished`
      (`KismetSystemLibrary.Delay` 0.001)
      (bind _output_get (set `self.Current Integer` (`KismetMathLibrary.RandomInteger` 11) :!label _label_2))
      (if (== (`self.Last Integer`) _output_get)
        (goto _label_2)
        (else
          (set `self.Last Integer` _current_integer)
          (goto _label))))))

(event `self.Sphere1.OnComponentBeginOverlap`
  (params (OverlappedComponent :type "PrimitiveComponent Object Reference") (OtherActor :type "Actor Object Reference") (OtherComp :type "PrimitiveComponent Object Reference") (OtherBodyIndex :type Integer) (bFromSweep :type Boolean) (SweepResult :type "HitResult Structure (by ref)"))
  (bind _returnvalue (`GameplayStatics.GetPlayerCharacter` 0))
  (if (== OtherActor _returnvalue)
    (bind _asbp_first_person_character (cast `/Game/Characters/Player/Animations/BP_FirstPersonCharacter` _returnvalue))
    (set `/Game/Characters/Player/Animations/BP_FirstPersonCharacter.Battery?` true _asbp_first_person_character)
    (`SceneComponent.SetVisibility` (`/Game/Characters/Player/Animations/BP_FirstPersonCharacter.Battery` _asbp_first_person_character) true false)
    (`self.K2_DestroyActor`)))

(fn `UserConstructionScript`)