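; Elevator Blueprint in the Battery Chase puzzle that lifts when the player character steps into its trigger box.
; The Box overlap waits briefly, then MoveComponentTo eases the Elevator component to the relative location in the Height variable.
; After a further delay, it eases the component back to zero relative location much faster, with all timing hardcoded in the event chain.
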(event `self.Box.OnComponentBeginOverlap`
  (params (OverlappedComponent :type "PrimitiveComponent Object Reference") (OtherActor :type "Actor Object Reference") (OtherComp :type "PrimitiveComponent Object Reference") (OtherBodyIndex :type Integer) (bFromSweep :type Boolean) (SweepResult :type "HitResult Structure (by ref)"))
  (if (== OtherActor (`GameplayStatics.GetPlayerCharacter` 0))
    (`KismetSystemLibrary.Delay` 0.2)
    (`KismetSystemLibrary.MoveComponentTo` (`self.Elevator`) (`self.Height`) (struct) true true 2.0)
    (`KismetSystemLibrary.Delay` 4.0)
    (`KismetSystemLibrary.MoveComponentTo` (`self.Elevator`) (0.0 0.0 0.0) (struct) true true 0.5)))

(fn `UserConstructionScript`)