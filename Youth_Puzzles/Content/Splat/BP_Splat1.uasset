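; BP_Splat1 is a splat decal actor with a Stick collision component that briefly interacts with the player.
; On BeginPlay, timed delays swap the decal through successive materials to animate the splat.
; Player overlap with Stick zeroes movement velocity after a short delay and destroys the splat, while overlap by an "energizer"-tagged actor destroys it immediately.
; Gravity-scale toggling for sticking is present but disconnected.
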(event `self.Stick.OnComponentBeginOverlap`
  (params (OverlappedComponent :type "PrimitiveComponent Object Reference") (OtherActor :type "Actor Object Reference") (OtherComp :type "PrimitiveComponent Object Reference") (OtherBodyIndex :type Integer) (bFromSweep :type Boolean) (SweepResult :type "HitResult Structure (by ref)"))
  (bind _returnvalue (`GameplayStatics.GetPlayerCharacter` 0))
  (if (== OtherActor _returnvalue)
    (bind _asbp_first_person_character (cast `/Game/Characters/Player/Animations/BP_FirstPersonCharacter` _returnvalue)
      (:`then`
        (`KismetSystemLibrary.Delay` 0.2)
        (set `MovementComponent.Velocity` (0.0 0.0 0.0) (`Character.CharacterMovement` _asbp_first_person_character))
        (`self.K2_DestroyActor`))
      (:`CastFailed`
        (`KismetSystemLibrary.PrintString` "CAST FAILED")))
    (elif (`self.ActorHasTag` OtherActor "energizer")
      (`self.K2_DestroyActor`))))

(event `self.Stick.OnComponentEndOverlap`
  (params (OverlappedComponent :type "PrimitiveComponent Object Reference") (OtherActor :type "Actor Object Reference") (OtherComp :type "PrimitiveComponent Object Reference") (OtherBodyIndex :type Integer)))

(event `self.ReceiveBeginPlay`
  (`KismetSystemLibrary.Delay` 0.2)
  (`DecalComponent.SetDecalMaterial` (`self.Decal`) "/Game/Splat/Splat_2.Splat_2")
  (`KismetSystemLibrary.Delay` 0.2)
  (`DecalComponent.SetDecalMaterial` (`self.Decal`) "/Game/Splat/Splat_3.Splat_3")
  (`KismetSystemLibrary.Delay` 0.2)
  (`DecalComponent.SetDecalMaterial` (`self.Decal`) "/Game/Splat/Splat_4.Splat_4"))

(fn `UserConstructionScript`)