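; BP_Goo is an actor that turns into a splat on impact.
; Each Tick adds a fixed yaw step to the energizer mesh, so its spin depends on frame rate.
; When the mesh registers a hit, it spawns BP_Splat at the mesh's location and rotation, then destroys itself.
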(event `self.ReceiveTick`
  (params (DeltaSeconds :type "Float (single-precision)"))
  (bind _energizer_mesh (`self.energizer_mesh`))
  (bind (_returnvalue_roll _returnvalue_pitch _returnvalue_yaw) (`KismetMathLibrary.BreakRotator` (`SceneComponent.K2_GetComponentRotation` _energizer_mesh)))
  (`SceneComponent.K2_SetWorldRotation` _energizer_mesh (`KismetMathLibrary.MakeRotator` _returnvalue_roll _returnvalue_pitch (+ _returnvalue_yaw 10.0)) false false))

(event `self.energizer_mesh.OnComponentHit`
  (params (HitComponent :type "PrimitiveComponent Object Reference") (OtherActor :type "Actor Object Reference") (OtherComp :type "PrimitiveComponent Object Reference") (NormalImpulse :type "Vector Structure") (Hit :type "HitResult Structure (by ref)"))
  (bind (_returnvalue_location _returnvalue_rotation) (`KismetMathLibrary.BreakTransform` (`SceneComponent.K2_GetComponentToWorld` (`self.energizer_mesh`))))
  (`|SpawnActorFromClass` "/Game/Splat/BP_Splat.BP_Splat_C" (`KismetMathLibrary.MakeTransform` _returnvalue_location _returnvalue_rotation) "AdjustIfPossibleButAlwaysSpawn" "OverrideRootScale" null null)
  (`self.K2_DestroyActor`))

(fn `UserConstructionScript`)