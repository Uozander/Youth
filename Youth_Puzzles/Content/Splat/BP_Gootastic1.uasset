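; Goo blob actor that leaves a BP_Splat where its sphere first hits something.
; On BeginPlay a short-delay loop keeps growing GOOMesh; the size limit is checked only once, and the Hit flag is never set by live logic.
; The first hit spawns a splat rotated to the surface normal and scaled from the mesh with a clamp, then destroys the actor after a brief delay.
; Stop-and-shrink logic is left disconnected.
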(event `self.ReceiveBeginPlay`
  (bind _goo_mesh (`self.GOO_mesh`))
  (bind _returnvalue (+ (`SceneComponent.RelativeScale3D` _goo_mesh) (0.1 0.1 0.1)))
  (if (<= (.x _returnvalue) 2.0)
    (if (not (`self.hit`)) :!label _label
      (`SceneComponent.SetRelativeScale3D` _goo_mesh _returnvalue)
      (`KismetSystemLibrary.Delay` 0.01)
      (goto _label))))

(event `self.Sphere.OnComponentHit`
  (params (HitComponent :type "PrimitiveComponent Object Reference") (OtherActor :type "Actor Object Reference") (OtherComp :type "PrimitiveComponent Object Reference") (NormalImpulse :type "Vector Structure") (Hit :type "HitResult Structure (by ref)"))
  (bind _returnvalue_location (`KismetMathLibrary.BreakTransform` (`SceneComponent.K2_GetComponentToWorld` (`self.Sphere`))))
  (bind (_returnvalue_roll _returnvalue_pitch _returnvalue_yaw) (`KismetMathLibrary.BreakRotator` (`KismetMathLibrary.Conv_VectorToRotator` (`.Normal` (`GameplayStatics.BreakHitResult` Hit)))))
  (`/Engine/EditorBlueprintResources/StandardMacros.DoOnce` false
    (:`Completed`
      (`|SpawnActorFromClass` "/Game/Splat/BP_Splat.BP_Splat_C" (`KismetMathLibrary.MakeTransform` _returnvalue_location (`KismetMathLibrary.MakeRotator` _returnvalue_roll _returnvalue_pitch _returnvalue_yaw) (`KismetMathLibrary.ClampVectorSize` (* (`SceneComponent.K2_GetComponentScale` (`self.GOO_mesh`)) (2.0 2.0 2.0)) 1.0 6.0)) "AdjustIfPossibleButAlwaysSpawn" "OverrideRootScale" null null)
      (`KismetSystemLibrary.Delay` 0.12)
      (`self.K2_DestroyActor`))))

(fn `UserConstructionScript`)