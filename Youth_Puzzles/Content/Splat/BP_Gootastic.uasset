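; BP_Gootastic is a goo blob actor that grows after spawning and turns into a splat on impact.
; BeginPlay uses a short Delay loop to enlarge GOOMesh step by step up to a size cap.
; The first Sphere hit on an actor not tagged "sticky" spawns a BP_Splat aligned to the surface normal and sized from the blob, then destroys the blob.
; Sticky hits only print a debug name, and the shrink-on-hit logic is disconnected.
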(event `self.ReceiveBeginPlay`
  (bind _goo_mesh (`self.GOO_mesh`))
  (bind _returnvalue (+ (`SceneComponent.RelativeScale3D` _goo_mesh) (0.1 0.1 0.1)))
  (if (<= (.x _returnvalue) 6.0) :!label _label
    (if (not (`self.hit`))
      (`SceneComponent.SetRelativeScale3D` _goo_mesh _returnvalue)
      (`KismetSystemLibrary.Delay` 0.01)
      (goto _label))))

(event `self.Sphere.OnComponentHit`
  (params (HitComponent :type "PrimitiveComponent Object Reference") (OtherActor :type "Actor Object Reference") (OtherComp :type "PrimitiveComponent Object Reference") (NormalImpulse :type "Vector Structure") (Hit :type "HitResult Structure (by ref)"))
  (bind (_bblockinghit _binitialoverlap _time _distance _location _impactpoint _normal _impactnormal) (`GameplayStatics.BreakHitResult` Hit))
  (if (`self.ActorHasTag` OtherActor "sticky")
    (`KismetSystemLibrary.PrintString` (`KismetSystemLibrary.GetDisplayName` OtherComp) true true (struct :`R` 1.0 :`G` 0.041493 :`A` 1.0))
    (else
      (`KismetSystemLibrary.PrintString` (`KismetSystemLibrary.GetDisplayName` OtherComp))
      (`/Engine/EditorBlueprintResources/StandardMacros.DoOnce` false
        (:`Completed`
          (bind _returnvalue (`|SpawnActorFromClass` "/Game/Splat/BP_Splat.BP_Splat_C" (`KismetMathLibrary.MakeTransform` _impactpoint (`KismetMathLibrary.Conv_VectorToRotator` _impactnormal) (`KismetMathLibrary.ClampVectorSize` (* (`SceneComponent.K2_GetComponentScale` (`self.GOO_mesh`)) (4.0 6.0 2.0)) 1.0 160.0)) "AdjustIfPossibleButAlwaysSpawn" "OverrideRootScale" null null))
          (`SceneComponent.SetRelativeScale3D` (`/Game/Splat/BP_Splat.Stick` _returnvalue) (1.0 0.01 1.0))
          (`KismetSystemLibrary.Delay` 0.12)
          (`self.K2_DestroyActor`))))))

(fn `UserConstructionScript`)