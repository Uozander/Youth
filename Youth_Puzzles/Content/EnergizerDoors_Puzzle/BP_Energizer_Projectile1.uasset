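; BP_Energizer_Projectile1 is a projectile actor, filed under the EnergizerDoors puzzle, that bursts on impact and removes itself.
; On a collision hit it prints the other actor's name, ignores the player character and itself, then spawns a burst effect at its collision component, oriented along the impact normal.
; It destroys itself after a short delay.
; The overlap event is empty, and a duplicate check chain is left unconnected.
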(event `self.energizer_collision.OnComponentBeginOverlap`
  (params (OverlappedComponent :type "PrimitiveComponent Object Reference") (OtherActor :type "Actor Object Reference") (OtherComp :type "PrimitiveComponent Object Reference") (OtherBodyIndex :type Integer) (bFromSweep :type Boolean) (SweepResult :type "HitResult Structure (by ref)")))

(event `self.energizer_collision1.OnComponentHit`
  (params (HitComponent :type "PrimitiveComponent Object Reference") (OtherActor :type "Actor Object Reference") (OtherComp :type "PrimitiveComponent Object Reference") (NormalImpulse :type "Vector Structure") (Hit :type "HitResult Structure (by ref)"))
  (bind _returnvalue_location (`KismetMathLibrary.BreakTransform` (`SceneComponent.K2_GetComponentToWorld` (`self.energizer_collision`))))
  (`KismetSystemLibrary.PrintString` (`KismetSystemLibrary.GetDisplayName` OtherActor))
  (if (!= OtherActor (`GameplayStatics.GetPlayerCharacter` 0))
    (if (!= OtherActor self)
      (`NiagaraFunctionLibrary.SpawnSystemAtLocation` "/Game/EnergizerDoors_Puzzle/Burst.Burst" _returnvalue_location (`KismetMathLibrary.Conv_VectorToRotator` (`.ImpactNormal` (`GameplayStatics.BreakHitResult` Hit))))
      (`KismetSystemLibrary.Delay` 0.2)
      (`self.K2_DestroyActor`))))

(fn `UserConstructionScript`)